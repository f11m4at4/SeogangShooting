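; BP_Enemy is an enemy actor that homes in on the player and destroys whatever it touches, along with itself.
; On BeginPlay it finds the BP_Player actor and stores it as Target.
; Each Tick it moves along the normalized direction to Target, scaled by Speed and delta time, without sweeping.
; When its Cube begins an overlap, it destroys the other actor and itself, with no type check.
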(event OnComponentBeginOverlap(Cube)
  (params (OverlappedComponent :type Primitive%20Component%20Object%20Reference) (OtherActor :type Actor%20Object%20Reference) (OtherComp :type Primitive%20Component%20Object%20Reference) (OtherBodyIndex :type Integer) (bFromSweep :type Boolean) (SweepResult :type Hit%20Result%20Structure%20%28by%20ref%29))
  (Actor|DestroyActor OtherActor)
  (Actor|DestroyActor))

(event EventBeginPlay
  (bind _returnvalue (Actor|GetActorOfClass "/Game/Blueprints/BP_Player.BP_Player_C"))
  (Variables|Default|SetTarget _returnvalue))

(event EventTick
  (params (DeltaSeconds :type Float%20%28single-precision%29))
  ;[1 1 1] 이동
  ;;[1 1 1] P
  (Transformation|SetActorLocation (+ (* (* (Variables|Default|GetSpeed) (Math|Vector|Normalize (- (Transformation|GetActorLocation (Variables|Default|GetTarget)) (Transformation|GetActorLocation)))) DeltaSeconds) (Transformation|GetActorLocation)) false false))

(fn ConstructionScript)