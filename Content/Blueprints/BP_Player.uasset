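; BP_Player is a player-controlled shooter that moves in the YZ plane and fires bullets.
; Each tick it builds a direction from the Horizontal and Vertical inputs, then moves by Speed times DeltaSeconds (P = P0 + vt) without sweeping.
; Two separate handlers for the Fire press spawn BP_Bullet at FirePosition and FirePosition1, with one also playing a blaster sound.
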(event EventTick
  (params (DeltaSeconds :type Float%20%28single-precision%29))
  ;[1 1 1] 방향구하기
  (Variables|Default|SetDirection (Math|Vector|MakeVector 0.0 (Input|AxisValues|GetHorizontal) (Input|AxisValues|GetVertical)))
  ;[1 1 1] P
  (Transformation|SetActorLocation (+ (* (* (Variables|Default|GetSpeed) (Variables|Default|GetDirection)) DeltaSeconds) (Transformation|GetActorLocation)) false false))

(event Input|ActionEvents|InputActionFire
  (params (Key :type Key%20Structure :default "None"))
  ;[1 1 1] 총알발사
  (:Pressed
    (Game|SpawnActorfromClass "/Game/Blueprints/BP_Bullet.BP_Bullet_C" (Transformation|GetWorldTransform (Variables|Default|GetFirePosition1)) "Undefined" 0 0)))

(event Input|ActionEvents|InputActionFire
  (params (Key :type Key%20Structure :default "None"))
  ;[1 1 1] 총알발사
  (:Pressed
    (Game|SpawnActorfromClass "/Game/Blueprints/BP_Bullet.BP_Bullet_C" (Transformation|GetWorldTransform (Variables|Default|GetFirePosition)) "Undefined" 0 0)
    (Audio|PlaySound2D "/Game/Audio/자료실_2장_star-wars-blaster__1_.자료실_2장_star-wars-blaster__1_" 1.0 1.0 0.0 0 0)))

(fn ConstructionScript)